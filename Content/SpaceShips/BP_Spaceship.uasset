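; BP_Spaceship is a spaceship actor with health, a regenerating shield and a status bar widget.
; Hurt lowers both values, spawns scattered floating damage numbers, and awards DefeatScore to BP_PlayerShip on every hit.
; A self-restarting timer, polled in Tick, re-enables shield regeneration after MinUnhurtTime without damage.
; At zero HP, Defeat spawns BP_Blast, awards score again and flags the actor for destruction on Tick.
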(event Custom|ResetHurtTimer
  (Utilities|Time|ClearandInvalidateTimerbyHandle (Variables|Default|GetUnhurtTimer))
  (bind _returnvalue (Utilities|Time|SetTimerbyEvent (delegate Custom|ResetHurtTimer) (Variables|Default|GetMinUnhurtTime) false true))
  (Variables|Default|SetUnhurtTimer _returnvalue))

(event EventBeginPlay
  (Variables|Default|SetToBeDestroyed false)
  (CallFunction|ResetHurtTimer)
  (Variables|Default|SetHP (Variables|Default|GetMaxHP))
  (Variables|Default|SetShield (Variables|Default|GetMaxShield))
  (Collision|SetActorEnableCollision true)
  (bind _aswb_status_bar (Utilities|Casting|CastToWB_StatusBar (UserInterface|GetWidget (Variables|Default|GetStatusBar))))
  (Rendering|Components|TextRender|SetText (Variables|/Game/GUI/WB_StatusBar.WB_StatusBar_C|GetName _aswb_status_bar) (Utilities|Text|ToText(String) (Variables|Default|GetName))))

(event Collision|EventActorBeginOverlap
  (params (OtherActor :type Actor%20Object%20Reference)))

(event EventTick
  (params (DeltaSeconds :type Float%20%28single-precision%29))
  (bind _maxshield (Variables|Default|GetMaxShield))
  (if (<= (Utilities|Time|GetTimerRemainingTimebyHandle (Variables|Default|GetUnhurtTimer)) 0.1)
    (Variables|Default|SetIsShieldIncreasing true))
  (if (Variables|Default|GetIsShieldIncreasing)
    (Class|ITakeDamage|Increase(Message) (UserInterface|GetWidget (Variables|Default|GetStatusBar)) (/ (Math|Float|Min(Float) (+ (Variables|Default|GetShield) (Variables|Default|GetDeltaShield)) _maxshield) _maxshield) (/ (Variables|Default|GetHP) (Variables|Default|GetMaxHP)))
    (Variables|Default|SetShield (Math|Float|Min(Float) (+ (Variables|Default|GetShield) (Variables|Default|GetDeltaShield)) _maxshield)))
  (if (Variables|Default|GetToBeDestroyed)
    (Actor|DestroyActor)))

(fn ConstructionScript)

(fn Defeat
  (params (BlastScale :type Vector))
  (bind _staticmesh (Variables|Default|GetStaticMesh))
  (bind _returnvalue (Transformation|GetWorldTransform _staticmesh))
  (Game|SpawnActorfromClass "/Game/Effects/BP_Blast.BP_Blast_C" (Math|Transform|MakeTransform (.location _returnvalue) (.rotation _returnvalue) BlastScale) "Undefined" "MultiplyWithRoot" 0 0)
  (Variables|Default|SetToBeDestroyed true)
  (bind _outactors (Actor|GetAllActorsOfClass "/Game/SpaceShips/Player/BP_PlayerShip.BP_PlayerShip_C"))
  (if (> (Utilities|Array|Length _outactors) 0)
    (Default|EarnScore (Utilities|Array|Get(acopy) _outactors) (Variables|Default|GetDefeatScore))))

(fn Hurt
  (params (DamageToShield :type Float%20%28double-precision%29) (DamageToHealth :type Float%20%28double-precision%29))
  (bind _statuscolor (Variables|Default|GetStatusColor))
  (CallFunction|ResetHurtTimer)
  (Variables|Default|SetIsShieldIncreasing false)
  (Variables|Default|SetShield (Math|Float|Max(Float) (- (Variables|Default|GetShield) DamageToShield) 0.0))
  (Variables|Default|SetHP (Math|Float|Max(Float) (- (Variables|Default|GetHP) DamageToHealth) 0.0))
  (if (> DamageToShield 0.0)
    (CallFunction|CreateDamageText DamageToShield (.shieldcolor _statuscolor)))
  (if (> DamageToHealth 0.0)
    (CallFunction|CreateDamageText DamageToHealth (.healthcolor _statuscolor)))
  (Class|ITakeDamage|Decay(Message) (UserInterface|GetWidget (Variables|Default|GetStatusBar)) (/ (Variables|Default|GetShield) (Variables|Default|GetMaxShield)) (/ (Variables|Default|GetHP) (Variables|Default|GetMaxHP)))
  (bind _outactors (Actor|GetAllActorsOfClass "/Game/SpaceShips/Player/BP_PlayerShip.BP_PlayerShip_C"))
  (if (> (Utilities|Array|Length _outactors) 0)
    (Default|EarnScore (Utilities|Array|Get(acopy) _outactors) (Variables|Default|GetDefeatScore)))
  (if (<= (Variables|Default|GetHP) 0.0)
    (CallFunction|Defeat "1.000000,1.000000,1.000000")))

(fn CreateDamageText
  (params (Damage :type Float%20%28double-precision%29) (Color :type Linear%20Color%20Structure) (Percision :type Integer))
  (bind _returnvalue (Game|GetPlayerController 0))
  (bind _returnvalue_2 (Math|Random|RandomUnitVector))
  (bind _returnvalue_3 (UserInterface|CreateWidget "/Game/GUI/WB_DamageDisplay.WB_DamageDisplay_C" _returnvalue))
  (UserInterface|Viewport|AddtoViewport _returnvalue_3 0)
  (Class|UserWidget|SetPositioninViewport _returnvalue_3 (+ (.ScreenPosition (Class|WidgetLayoutLibrary|ProjectWorldLocationtoWidgetPosition _returnvalue (.location (Transformation|GetWorldTransform (Variables|Default|GetStatusBar self))) false)) (* (Math|Vector2D|MakeVector2D (.x _returnvalue_2) (.y _returnvalue_2)) (Math|Random|RandomFloatinRange 0.0 5e+01))) false)
  (Class|IDisplayDamage|DisplayDamage(Message) _returnvalue_3 Damage Color Percision))