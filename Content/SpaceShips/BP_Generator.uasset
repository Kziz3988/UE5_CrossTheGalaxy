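; Spawner actor that generates waves of enemy fighters and cruisers, cycling endlessly through predefined swarm compositions.
; The Construction Script fills the ship class list and the swarms, each holding class indices and an interval.
; Tick spawns the active swarm, then polls a timer used as countdown, clearing it just before expiry to advance the index and restart.
; Each ship spawns far along X at randomized Y/Z offsets, yawed or turned around.
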(event Custom|FinishInterval
  (Variables|Default|SetIsEnabled false)
  (Utilities|Time|ClearandInvalidateTimerbyHandle (Variables|Default|GetCloneTimer)))

(event Custom|BeginInterval
  (bind _returnvalue (Utilities|Time|SetTimerbyEvent (delegate Custom|BeginInterval) (.interval (Utilities|Array|Get(acopy) (Variables|Default|GetSwarms) (Variables|Default|GetActiveIndex)))))
  (Variables|Default|SetCloneTimer _returnvalue))

(event EventBeginPlay)

(event Collision|EventActorBeginOverlap
  (params (OtherActor :type Actor%20Object%20Reference)))

(event EventTick
  (params (DeltaSeconds :type Float%20%28single-precision%29))
  (if (Variables|Default|GetIsEnabled)
    (if (<= (Utilities|Time|GetTimerRemainingTimebyHandle (Variables|Default|GetCloneTimer)) 0.1)
      (CallFunction|CloneSwarm false))
    (else
      (CallFunction|CloneSwarm true)
      (Variables|Default|SetIsEnabled true))))

(fn ConstructionScript
  (Variables|Default|SetSpaceships (Utilities|Array|MakeArray "/Game/SpaceShips/Enemy/BP_EnemyFighter1.BP_EnemyFighter1_C" "/Game/SpaceShips/Enemy/BP_EnemyFighter2.BP_EnemyFighter2_C" "/Game/SpaceShips/Enemy/BP_EnemyCruiser1.BP_EnemyCruiser1_C" "/Game/SpaceShips/Enemy/BP_EnemyCruiser2.BP_EnemyCruiser2_C"))
  (Variables|Default|SetSwarms (Utilities|Array|MakeArray (Utilities|Struct|MakeDS_EnemySwarm (Utilities|Array|MakeArray 0 0 0 0) 5.0) (Utilities|Struct|MakeDS_EnemySwarm (Utilities|Array|MakeArray 1 1 1) 5.0) (Utilities|Struct|MakeDS_EnemySwarm (Utilities|Array|MakeArray 2 2 0 0) 5.0) (Utilities|Struct|MakeDS_EnemySwarm (Utilities|Array|MakeArray 3 0 0) 5.0))))

(fn CloneSwarm
  (params (IsEnabled :type Boolean))
  (if IsEnabled
    (for _array_element (.spaceships (Utilities|Array|Get(acopy) (Variables|Default|GetSwarms) (Variables|Default|GetActiveIndex)))
      (CallFunction|CloneSpaceship (Utilities|Array|Get(acopy) (Variables|Default|GetSpaceships) _array_element)))
    (else
      (CallFunction|FinishInterval)
      (Variables|Default|SetActiveIndex (Math|Integer|%(Integer) (+ (Variables|Default|GetActiveIndex) 1) (Utilities|Array|Length (Variables|Default|GetSwarms))))
      (CallFunction|BeginInterval))))

(fn CloneSpaceship
  (params (Spaceship :type Pawn%20Class%20Reference))
  (bind _returnvalue (Math|Random|RandomUnitVector))
  (bind _returnvalue_2 (* _returnvalue 5e+03))
  (Game|SpawnActorfromClass Spaceship (Math|Transform|MakeTransform (Math|Vector|MakeVector 5e+04 (.y _returnvalue_2) (+ (.z _returnvalue_2) 1e+04)) "180.000000,0.000000,0.000000" "1.000000,1.000000,1.000000") "Undefined" "MultiplyWithRoot" 0 0))