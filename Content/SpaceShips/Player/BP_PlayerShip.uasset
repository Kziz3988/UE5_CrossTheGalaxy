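; Player-controlled spaceship pawn that moves up, down and sideways within bounds, with forward and rotation input disabled.
; Tick clamps the mesh's Y/Z position, derives roll and pitch from it, and runs booster trails that follow sideways input.
; Enhanced Input toggles paired machine gun and laser child actors.
; Hurt updates shield, health and status bar, awards DefeatScore on every hit, and at zero HP shows WB_PauseMenu with the score before Defeat.
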(event Input|EnhancedActionEvents|EnhancedInputActionIA_MoveForward_CC
  (params (ActionValue :type Float%20%28double-precision%29) (ElapsedSeconds :type Float%20%28double-precision%29) (TriggeredSeconds :type Float%20%28double-precision%29) (InputAction :type Input%20Action%20Object%20Reference :default "/Game/Input/IA_MoveForward_CC.IA_MoveForward_CC"))
  (Pawn|Input|AddMovementInput (Math|Vector|GetForwardVector (Pawn|GetControlRotation :!class /Script/Engine.Pawn)) ActionValue false))

(event Input|EnhancedActionEvents|EnhancedInputActionIA_MoveUp_CC
  (params (ActionValue :type Float%20%28double-precision%29) (ElapsedSeconds :type Float%20%28double-precision%29) (TriggeredSeconds :type Float%20%28double-precision%29) (InputAction :type Input%20Action%20Object%20Reference :default "/Game/Input/IA_MoveUp_CC.IA_MoveUp_CC"))
  (Pawn|Input|AddMovementInput (Math|Vector|GetUpVector (Pawn|GetControlRotation :!class /Script/Engine.Pawn)) ActionValue false))

(event Input|EnhancedActionEvents|EnhancedInputActionIA_MoveRight_CC
  (params (ActionValue :type Float%20%28double-precision%29) (ElapsedSeconds :type Float%20%28double-precision%29) (TriggeredSeconds :type Float%20%28double-precision%29) (InputAction :type Input%20Action%20Object%20Reference :default "/Game/Input/IA_MoveRight_CC.IA_MoveRight_CC"))
  (Pawn|Input|AddMovementInput (Math|Vector|GetRightVector (Pawn|GetControlRotation :!class /Script/Engine.Pawn)) ActionValue false))

(event Input|EnhancedActionEvents|EnhancedInputActionIA_SwitchLaser
  (params (ActionValue :type Boolean) (ElapsedSeconds :type Float%20%28double-precision%29) (TriggeredSeconds :type Float%20%28double-precision%29) (InputAction :type Input%20Action%20Object%20Reference :default "/Game/Input/IA_SwitchLaser.IA_SwitchLaser"))
  (bind _laser_gun_l (Variables|Default|GetLaser_Gun_L))
  (bind _laser_gun_r (Variables|Default|GetLaser_Gun_R))
  (bind _childactor (Variables|/Script/Engine.ChildActorComponent|GetChildActor _laser_gun_l))
  (bind _childactor_2 (Variables|/Script/Engine.ChildActorComponent|GetChildActor _laser_gun_r))
  (:Triggered
    (Class|IWeapon|Switch(Message) _childactor true)
    (Class|IWeapon|Switch(Message) _childactor_2 true))
  (:Completed
    (Class|IWeapon|Switch(Message) _childactor false)
    (Class|IWeapon|Switch(Message) _childactor_2 false)))

(event Input|EnhancedActionEvents|EnhancedInputActionIA_RotateYaw_CC
  (params (ActionValue :type Float%20%28double-precision%29) (ElapsedSeconds :type Float%20%28double-precision%29) (TriggeredSeconds :type Float%20%28double-precision%29) (InputAction :type Input%20Action%20Object%20Reference :default "/Game/Input/IA_RotateYaw_CC.IA_RotateYaw_CC"))
  (Pawn|Input|AddControllerYawInput ActionValue))

(event Input|EnhancedActionEvents|EnhancedInputActionIA_RotatePitch_CC
  (params (ActionValue :type Float%20%28double-precision%29) (ElapsedSeconds :type Float%20%28double-precision%29) (TriggeredSeconds :type Float%20%28double-precision%29) (InputAction :type Input%20Action%20Object%20Reference :default "/Game/Input/IA_RotatePitch_CC.IA_RotatePitch_CC"))
  (Pawn|Input|AddControllerPitchInput ActionValue))

(event Input|EnhancedActionEvents|EnhancedInputActionIA_SwitchGun
  (params (ActionValue :type Boolean) (ElapsedSeconds :type Float%20%28double-precision%29) (TriggeredSeconds :type Float%20%28double-precision%29) (InputAction :type Input%20Action%20Object%20Reference :default "/Game/Input/IA_SwitchGun.IA_SwitchGun"))
  (bind _machine_gun_l (Variables|Default|GetMachine_Gun_L))
  (bind _machine_gun_r (Variables|Default|GetMachine_Gun_R))
  (bind _childactor (Variables|/Script/Engine.ChildActorComponent|GetChildActor _machine_gun_r))
  (bind _childactor_2 (Variables|/Script/Engine.ChildActorComponent|GetChildActor _machine_gun_l))
  (:Triggered
    (Class|IWeapon|Switch(Message) _childactor_2 true)
    (Class|IWeapon|Switch(Message) _childactor true))
  (:Completed
    (Class|IWeapon|Switch(Message) _childactor_2 false)
    (Class|IWeapon|Switch(Message) _childactor false)))

(event EventBeginPlay
  (|CallParentFunction)
  (Collision|SetActorEnableCollision true))

(event Collision|EventActorBeginOverlap
  (params (OtherActor :type Actor%20Object%20Reference))
  (|CallParentFunction OtherActor))

(event EventTick
  (params (DeltaSeconds :type Float%20%28single-precision%29))
  (bind _staticmesh (Variables|Default|GetStaticMesh))
  (bind _zmax (Variables|Default|GetZMax))
  (bind _zmin (Variables|Default|GetZMin))
  (bind _ymax (Variables|Default|GetYMax))
  (bind _ymin (Variables|Default|GetYMin))
  (bind _returnvalue (Transformation|GetWorldLocation _staticmesh))
  (bind _returnvalue_2 (- _zmax _zmin))
  (bind _returnvalue_3 (- _ymax _ymin))
  (bind _returnvalue_4 (Math|Float|Clamp(Float) (.z _returnvalue) _zmin _zmax))
  (bind _returnvalue_5 (Math|Float|Clamp(Float) (.y _returnvalue) _ymin _ymax))
  (bind _returnvalue_6 (/ _returnvalue_2 2.0))
  (|CallParentFunction DeltaSeconds)
  (if (not (Variables|Default|GetToBeDestroyed))
    (CallFunction|SwitchBooster true)
    (Transformation|SetWorldLocationAndRotation (Variables|Default|GetStaticMesh) (Math|Vector|MakeVector 0.0 _returnvalue_5 _returnvalue_4) (Math|Rotator|MakeRotator (* (/ (- (/ _returnvalue_3 2.0) (- _returnvalue_5 _ymin)) _returnvalue_3) 15.0) (* (/ (- _returnvalue_6 (- _returnvalue_4 _zmin)) _returnvalue_6) 15.0) 0.0) false false)))

(event EventPossessed
  (params (NewController :type Controller%20Object%20Reference))
  (bind _aspc_spaceship (Utilities|Casting|CastToPC_Spaceship NewController))
  (Input|AddMappingContext (PlayerController|LocalPlayerSubsystems|GetEnhancedInputLocalPlayerSubsystem _aspc_spaceship) "/Game/Input/IMC_Spaceship.IMC_Spaceship" 0 "(bIgnoreAllPressedKeysUntilRelease=True,bForceImmediately=False,bNotifyUserSettings=False)"))

(fn ConstructionScript)

(fn SwitchBooster
  (params (isActive :type Boolean))
  (if isActive
    (Components|Activation|Activate (Variables|Default|GetNS_Trail_1) false)
    (CallFunction|SwitchSideBooster isActive)
    (else
      (Components|Activation|Deactivate (Variables|Default|GetNS_Trail_1))
      (CallFunction|SwitchSideBooster isActive))))

(fn SwitchSideBooster
  (params (isActive :type Boolean))
  (bind _returnvalue (Input|EnhancedActionValues|GetIA_MoveRight_CC))
  (if (== _returnvalue 0.0)
    (Components|Activation|Activate (Variables|Default|GetNS_SideTrail_L) false)
    (Components|Activation|Activate (Variables|Default|GetNS_SideTrail_R) false)
    (elif (< 0.0 _returnvalue)
      (Components|Activation|Activate (Variables|Default|GetNS_SideTrail_L) false)
      (Components|Activation|Deactivate (Variables|Default|GetNS_SideTrail_R))
      (else
        (Components|Activation|Activate (Variables|Default|GetNS_SideTrail_R) false)
        (Components|Activation|Deactivate (Variables|Default|GetNS_SideTrail_L))))))

(fn EarnScore
  (params (Score :type Integer))
  (bind _output_get (Variables|Default|SetScore Score))
  (bind _aswb_player_status_bar (Utilities|Casting|CastToWB_PlayerStatusBar (UserInterface|GetWidget (Variables|Default|GetStatusBar))))
  (Default|EarnScore _aswb_player_status_bar _output_get))

(fn Hurt
  (params (DamageToShield :type Float%20%28double-precision%29) (DamageToHealth :type Float%20%28double-precision%29))
  (CallFunction|ResetHurtTimer)
  (Variables|Default|SetIsShieldIncreasing false)
  (Variables|Default|SetShield (Math|Float|Max(Float) (- (Variables|Default|GetShield) DamageToShield) 0.0))
  (Variables|Default|SetHP (Math|Float|Max(Float) (- (Variables|Default|GetHP) DamageToHealth) 0.0))
  (Class|ITakeDamage|Decay(Message) (UserInterface|GetWidget (Variables|Default|GetStatusBar)) (/ (Variables|Default|GetShield) (Variables|Default|GetMaxShield)) (/ (Variables|Default|GetHP) (Variables|Default|GetMaxHP)))
  (bind _outactors (Actor|GetAllActorsOfClass "BP_PlayerShip_C"))
  (if (> (Utilities|Array|Length _outactors) 0)
    (CallFunction|EarnScore (Utilities|Array|Get(acopy) _outactors) (Variables|Default|GetDefeatScore)))
  (if (<= (Variables|Default|GetHP) 0.0)
    (bind _returnvalue (Game|ConstructObjectfromClass "/Game/GUI/WB_PauseMenu.WB_PauseMenu_C"))
    (UserInterface|Viewport|AddtoViewport _returnvalue 0)
    (bind _aswb_player_status_bar (Utilities|Casting|CastToWB_PlayerStatusBar (UserInterface|GetWidget (Variables|Default|GetStatusBar))))
    (Rendering|Components|TextRender|SetText (Variables|/Game/GUI/WB_PauseMenu.WB_PauseMenu_C|GetScore _returnvalue) (Class|TextBlock|GetText (Variables|/Game/GUI/WB_PlayerStatusBar.WB_PlayerStatusBar_C|GetScore _aswb_player_status_bar)))
    (Variables|/Script/Engine.PlayerController|SetbShowMouseCursor (Game|GetPlayerController 0) true)
    (CallFunction|Defeat "1.000000,1.000000,1.000000")))