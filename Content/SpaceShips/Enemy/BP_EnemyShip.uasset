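; Enemy spaceship that moves along its mesh's forward vector while cycling through the weapon sets in its AttackStrategy array.
; A timer set for each entry's Duration calls Fire, which switches those weapons off, advances the index with wraparound and restarts the timer.
; Tick switches on the current set whenever IsEnabled is false, otherwise moves the ship and sets ToBeDestroyed once mesh relative X drops below zero.
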(event Custom|FinishAttack
  (Variables|Default|SetIsEnabled false)
  (Utilities|Time|ClearandInvalidateTimerbyHandle (Variables|Default|GetAttackTimer)))

(event Custom|Fire
  (CallFunction|SwitchWeapons false (.weapons (Utilities|Array|Get(acopy) (Variables|Default|GetAttackStrategy) (Variables|Default|GetActiveIndex)))))

(event Custom|BeginAttack
  (bind _returnvalue (Utilities|Time|SetTimerbyEvent (delegate Custom|Fire) (.duration (Utilities|Array|Get(acopy) (Variables|Default|GetAttackStrategy) (Variables|Default|GetActiveIndex)))))
  (Variables|Default|SetAttackTimer _returnvalue))

(event EventBeginPlay
  (|CallParentFunction))

(event Collision|EventActorBeginOverlap
  (params (OtherActor :type Actor%20Object%20Reference))
  (|CallParentFunction OtherActor) ; 此节点被禁用，将不会被调用。\n从引脚连出引线来编译功能。
)

(event EventTick
  (params (DeltaSeconds :type Float%20%28single-precision%29))
  (|CallParentFunction DeltaSeconds)
  (if (not (Variables|Default|GetToBeDestroyed))
    (if (Variables|Default|GetIsEnabled)
      (Pawn|Input|AddMovementInput (Math|Vector|GetForwardVector (.rotation (Transformation|GetRelativeTransform (Variables|Default|GetStaticMesh)))) (Variables|Default|GetSpeed) false)
      (if (< (.x (.location (Transformation|GetRelativeTransform (Variables|Default|GetStaticMesh)))) 0.0)
        (Variables|Default|SetToBeDestroyed true))
      (else
        (CallFunction|SwitchWeapons true (.weapons (Utilities|Array|Get(acopy) (Variables|Default|GetAttackStrategy) (Variables|Default|GetActiveIndex))))
        (Variables|Default|SetIsEnabled true)))))

(fn ConstructionScript
  (|CallParentFunction))

(fn SwitchWeapons
  (params (IsEnabled :type Boolean) (Weapons :type Array%20of%20Actor%20Object%20References))
  (if IsEnabled
    (for _array_element Weapons
      (Class|IWeapon|Switch(Message) _array_element true))
    (else
      (CallFunction|FinishAttack)
      (for _array_element_2 Weapons
        (Class|IWeapon|Switch(Message) _array_element_2 false))
      (Variables|Default|SetActiveIndex (Math|Integer|%(Integer) (+ (Variables|Default|GetActiveIndex) 1) (Utilities|Array|Length (Variables|Default|GetAttackStrategy))))
      (CallFunction|BeginAttack))))