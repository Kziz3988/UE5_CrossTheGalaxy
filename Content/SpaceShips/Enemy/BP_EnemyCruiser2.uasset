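; BP_EnemyCruiser2 is an enemy cruiser spaceship that configures its weapon attack pattern on top of inherited behavior.
; On BeginPlay it adds three AttackStrategy phases of equal timing: four laser guns, two lasers with two machine guns, then an empty weapon set.
; It then calls SwitchWeapons to enable the weapons at ActiveIndex.
; Weapons are child actor components, and this graph contains no logic for advancing phases.
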(event Collision|EventActorBeginOverlap
  (params (OtherActor :type Actor%20Object%20Reference))
  (|CallParentFunction OtherActor) ; 此节点被禁用，将不会被调用。\n从引脚连出引线来编译功能。
)

(event EventTick
  (params (DeltaSeconds :type Float%20%28single-precision%29))
  (|CallParentFunction DeltaSeconds) ; 此节点被禁用，将不会被调用。\n从引脚连出引线来编译功能。
)

(event EventBeginPlay
  (|CallParentFunction)
  (Utilities|Array|Add (Variables|Default|GetAttackStrategy) (Utilities|Struct|MakeDS_EnemyAttack (Utilities|Array|MakeArray (Variables|/Script/Engine.ChildActorComponent|GetChildActor (Variables|Default|GetLaser_Gun_L1)) (Variables|/Script/Engine.ChildActorComponent|GetChildActor (Variables|Default|GetLaser_Gun_L2)) (Variables|/Script/Engine.ChildActorComponent|GetChildActor (Variables|Default|GetLaser_Gun_R1)) (Variables|/Script/Engine.ChildActorComponent|GetChildActor (Variables|Default|GetLaser_Gun_R2))) 1.5))
  (Utilities|Array|Add (Variables|Default|GetAttackStrategy) (Utilities|Struct|MakeDS_EnemyAttack (Utilities|Array|MakeArray (Variables|/Script/Engine.ChildActorComponent|GetChildActor (Variables|Default|GetLaser_Gun_L3)) (Variables|/Script/Engine.ChildActorComponent|GetChildActor (Variables|Default|GetLaser_Gun_R3)) (Variables|/Script/Engine.ChildActorComponent|GetChildActor (Variables|Default|GetMachine_Gun_L)) (Variables|/Script/Engine.ChildActorComponent|GetChildActor (Variables|Default|GetMachine_Gun_R))) 1.5))
  (Utilities|Array|Add (Variables|Default|GetAttackStrategy) (Utilities|Struct|MakeDS_EnemyAttack "(None)" 1.5))
  (CallFunction|SwitchWeapons true (.weapons (Utilities|Array|Get(acopy) (Variables|Default|GetAttackStrategy) (Variables|Default|GetActiveIndex)))))

(fn ConstructionScript
  (|CallParentFunction))