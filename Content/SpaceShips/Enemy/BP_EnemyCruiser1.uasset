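; Enemy cruiser ship Blueprint that defines its weapon attack pattern on top of inherited parent behavior.
; On BeginPlay it fills AttackStrategy with three phases, each pairing a weapon set with a number, likely a duration: machine guns plus four lasers, lasers only, then no weapons.
; It then enables the active phase's weapons through SwitchWeapons.
; Construction, overlap and tick only call the parent.
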(event Collision|EventActorBeginOverlap
  (params (OtherActor :type Actor%20Object%20Reference))
  (|CallParentFunction OtherActor))

(event EventTick
  (params (DeltaSeconds :type Float%20%28single-precision%29))
  (|CallParentFunction DeltaSeconds))

(event EventBeginPlay
  (|CallParentFunction)
  (Utilities|Array|Add (Variables|Default|GetAttackStrategy) (Utilities|Struct|MakeDS_EnemyAttack (Utilities|Array|MakeArray (Variables|/Script/Engine.ChildActorComponent|GetChildActor (Variables|Default|GetMachine_Gun_L)) (Variables|/Script/Engine.ChildActorComponent|GetChildActor (Variables|Default|GetMachine_Gun_R)) (Variables|/Script/Engine.ChildActorComponent|GetChildActor (Variables|Default|GetLaser_Front_L)) (Variables|/Script/Engine.ChildActorComponent|GetChildActor (Variables|Default|GetLaser_Front_R)) (Variables|/Script/Engine.ChildActorComponent|GetChildActor (Variables|Default|GetLaser_Back_L)) (Variables|/Script/Engine.ChildActorComponent|GetChildActor (Variables|Default|GetLaser_Back_R))) 1.5))
  (Utilities|Array|Add (Variables|Default|GetAttackStrategy) (Utilities|Struct|MakeDS_EnemyAttack (Utilities|Array|MakeArray (Variables|/Script/Engine.ChildActorComponent|GetChildActor (Variables|Default|GetLaser_Front_L)) (Variables|/Script/Engine.ChildActorComponent|GetChildActor (Variables|Default|GetLaser_Front_R)) (Variables|/Script/Engine.ChildActorComponent|GetChildActor (Variables|Default|GetLaser_Back_L)) (Variables|/Script/Engine.ChildActorComponent|GetChildActor (Variables|Default|GetLaser_Back_R))) 2.0))
  (Utilities|Array|Add (Variables|Default|GetAttackStrategy) (Utilities|Struct|MakeDS_EnemyAttack "(None)" 1.0))
  (CallFunction|SwitchWeapons true (.weapons (Utilities|Array|Get(acopy) (Variables|Default|GetAttackStrategy) (Variables|Default|GetActiveIndex)))))

(fn ConstructionScript
  (|CallParentFunction))