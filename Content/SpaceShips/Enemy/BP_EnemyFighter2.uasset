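; BP_EnemyFighter2 is an enemy spaceship fighter that configures its own weapon attack pattern on top of inherited parent behavior.
; On BeginPlay it fills AttackStrategy with a timed phase using the left and right laser child actors, then a shorter phase with no weapons.
; It then calls SwitchWeapons to enable the weapons of the active strategy entry.
; Overlap, Tick and construction add no logic of their own.
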(event EventBeginPlay
  (|CallParentFunction)
  (Utilities|Array|Add (Variables|Default|GetAttackStrategy) (Utilities|Struct|MakeDS_EnemyAttack (Utilities|Array|MakeArray (Variables|/Script/Engine.ChildActorComponent|GetChildActor (Variables|Default|GetLaser_L)) (Variables|/Script/Engine.ChildActorComponent|GetChildActor (Variables|Default|GetLaser_R))) 3.5))
  (Utilities|Array|Add (Variables|Default|GetAttackStrategy) (Utilities|Struct|MakeDS_EnemyAttack "(None)" 1.5))
  (CallFunction|SwitchWeapons true (.weapons (Utilities|Array|Get(acopy) (Variables|Default|GetAttackStrategy) (Variables|Default|GetActiveIndex)))))

(event Collision|EventActorBeginOverlap
  (params (OtherActor :type Actor%20Object%20Reference))
  (|CallParentFunction OtherActor) ; 此节点被禁用，将不会被调用。\n从引脚连出引线来编译功能。
)

(event EventTick
  (params (DeltaSeconds :type Float%20%28single-precision%29))
  (|CallParentFunction DeltaSeconds) ; 此节点被禁用，将不会被调用。\n从引脚连出引线来编译功能。
)

(fn ConstructionScript
  (|CallParentFunction))