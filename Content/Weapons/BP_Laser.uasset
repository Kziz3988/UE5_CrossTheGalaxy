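; Switchable laser weapon that traces a beam from its gun and damages any BP_Spaceship it hits.
; While enabled, a looping timer line-traces along the gun's up vector, ignoring actors with a configurable tag.
; The beam mesh is Z-scaled to the hit distance or maximum range, and zero-scaled when off.
; On a hit, the ship's status bar widget splits damage between shield and health before Hurt applies it.
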(event Custom|LaserSwitchedOn
  (bind _returnvalue (Utilities|Time|SetTimerbyEvent (delegate Custom|Fire) (Variables|Default|GetLaserCycle) true true))
  (Variables|Default|SetLaserTimer _returnvalue))

(event Custom|LaserSwitchedOff
  (Utilities|Time|ClearandInvalidateTimerbyHandle (Variables|Default|GetLaserTimer)))

(event Custom|Fire
  (CallFunction|SetLaserRange (Variables|Default|GetTagIgnore)))

(event EventBeginPlay
  (CallFunction|SwitchLaser false))

(event Collision|EventActorBeginOverlap
  (params (OtherActor :type Actor%20Object%20Reference)))

(event EventSwitch
  (params (IsEnabled :type Boolean))
  (CallFunction|SwitchLaser IsEnabled))

(fn ConstructionScript)

(fn SwitchLaser
  (params (IsEnabled :type Boolean))
  (if IsEnabled
    (if (not (Variables|Default|GetIsLaserEnabled))
      (Variables|Default|SetIsLaserEnabled true)
      (CallFunction|LaserSwitchedon))
    (else
      (Transformation|SetRelativeScale3D (Variables|Default|GetLaser) "0, 0, 0")
      (Variables|Default|SetIsLaserEnabled false)
      (CallFunction|LaserSwitchedOff))))

(fn SetLaserRange
  (params (TagIgnore :type String))
  (bind _laser (Variables|Default|GetLaser))
  (bind _maxlaserrange (Variables|Default|GetMaxLaserRange))
  (bind _laser_gun (Variables|Default|GetLaser_Gun))
  (bind _returnvalue (Transformation|GetWorldTransform _laser_gun))
  (bind _outactors (Actor|GetAllActorswithTag (Utilities|String|StringToName TagIgnore)))
  (bind (_outhit _returnvalue_2) (Collision|LineTraceByChannel (.location _returnvalue) (+ (.location _returnvalue) (* (Math|Vector|GetUpVector (.rotation _returnvalue)) (Variables|Default|GetMaxLaserRange))) "TraceTypeQuery1" false _outactors "None"))
  (if _returnvalue_2
    (Transformation|SetRelativeScale3D _laser (Math|Vector|MakeVector 1e+01 1e+01 (Math|Float|Min(Float) _maxlaserrange (Math|Vector|Distance(Vector) (.location _returnvalue) (.ImpactPoint (Collision|BreakHitResult _outhit))))))
    (bind _asbp_spaceship (Utilities|Casting|CastToBP_Spaceship (.HitActor (Collision|BreakHitResult _outhit))))
    (Utilities|FlowControl|DoOnce false
      (:Completed
        (bind (_damagetoshield _damagetohealth) (Class|ITakeDamage|TakeDamage(Message) (UserInterface|GetWidget (Variables|/Game/SpaceShips/BP_Spaceship.BP_Spaceship_C|GetStatusBar _asbp_spaceship)) (Variables|/Game/SpaceShips/BP_Spaceship.BP_Spaceship_C|GetShield _asbp_spaceship) (Variables|/Game/SpaceShips/BP_Spaceship.BP_Spaceship_C|GetHP _asbp_spaceship) (Variables|/Game/SpaceShips/BP_Spaceship.BP_Spaceship_C|GetArmor _asbp_spaceship) (Variables|Default|GetDamage)))
        (Default|Hurt _asbp_spaceship _damagetoshield _damagetohealth)))
    (else
      (Transformation|SetRelativeScale3D _laser (Math|Vector|MakeVector 1e+01 1e+01 _maxlaserrange)))))

(fn SetLaserData
  (params (LaserCycle :type Float%20%28double-precision%29) (LaserRange :type Float%20%28double-precision%29) (Damage :type DS%20Damage%20Structure) (TagIgnore :type String) (Material :type Material%20Instance%20Object%20Reference))
  (Variables|Default|SetLaserCycle LaserCycle)
  (Variables|Default|SetMaxLaserRange LaserRange)
  (Variables|Default|SetDamage Damage)
  (Variables|Default|SetTagIgnore TagIgnore)
  (Rendering|Material|SetMaterial (Variables|Default|GetLaser) 0 Material))