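; Projectile that flies forward and damages the first BP_Spaceship it overlaps whose first tag matches TargetTag.
; Tick sweeps the mesh along its forward vector using its own speed plus a scaled gun speed from SetSpeed.
; On a hit, the target's status bar widget splits damage into shield and health amounts for Hurt.
; The bullet destroys itself after a hit, beyond MaxDistance from the player ship, at negative relative X, or without a player.
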(event OnComponentBeginOverlap(StaticMesh)
  (params (OverlappedComponent :type Primitive%20Component%20Object%20Reference) (OtherActor :type Actor%20Object%20Reference) (OtherComp :type Primitive%20Component%20Object%20Reference) (OtherBodyIndex :type Integer) (bFromSweep :type Boolean) (SweepResult :type Hit%20Result%20Structure%20%28by%20ref%29))
  (if (not (Variables|Default|GetToBeDestroyed))
    (if (== (Utilities|Array|Get(acopy) (Variables|/Script/Engine.Actor|GetTags OtherActor)) (Variables|Default|GetTargetTag))
      (bind _asbp_spaceship (Utilities|Casting|CastToBP_Spaceship OtherActor))
      (Utilities|FlowControl|DoOnce false
        (:Completed
          (bind (_damagetoshield _damagetohealth) (Class|ITakeDamage|TakeDamage(Message) (UserInterface|GetWidget (Variables|/Game/SpaceShips/BP_Spaceship.BP_Spaceship_C|GetStatusBar _asbp_spaceship)) (Variables|/Game/SpaceShips/BP_Spaceship.BP_Spaceship_C|GetShield _asbp_spaceship) (Variables|/Game/SpaceShips/BP_Spaceship.BP_Spaceship_C|GetHP _asbp_spaceship) (Variables|/Game/SpaceShips/BP_Spaceship.BP_Spaceship_C|GetArmor _asbp_spaceship) (Variables|Default|GetDamage)))
          (Default|Hurt _asbp_spaceship _damagetoshield _damagetohealth)
          (Variables|Default|SetToBeDestroyed true))))))

(event Custom|SetSpeed
  (params (GunSpeed :type Float%20%28double-precision%29))
  (Variables|Default|SetGunSpeed (* GunSpeed 0.1))
  (Transformation|SetMobility (Variables|Default|GetStaticMesh) "Movable"))

(event EventBeginPlay
  (Variables|Default|SetToBeDestroyed false))

(event Collision|EventActorBeginOverlap
  (params (OtherActor :type Actor%20Object%20Reference)))

(event EventTick
  (params (DeltaSeconds :type Float%20%28single-precision%29))
  (bind _staticmesh (Variables|Default|GetStaticMesh))
  (bind _returnvalue (Transformation|GetRelativeTransform _staticmesh))
  (Transformation|SetRelativeTransform (Variables|Default|GetStaticMesh) (Math|Transform|MakeTransform (+ (.location _returnvalue) (* (Math|Vector|GetForwardVector (.rotation _returnvalue)) (+ (Variables|Default|GetGunSpeed) (Variables|Default|GetSpeed)))) (.rotation _returnvalue) (.scale _returnvalue)) true false)
  (bind _outactors (Actor|GetAllActorsOfClass "/Game/SpaceShips/Player/BP_PlayerShip.BP_PlayerShip_C"))
  (if (> (Utilities|Array|Length _outactors) 0)
    (if (or (> (Math|Vector|Distance(Vector) (Transformation|GetActorLocation (Utilities|Array|Get(acopy) _outactors)) (Transformation|GetWorldLocation (Variables|Default|GetStaticMesh))) (Variables|Default|GetMaxDistance)) (or (< (.x (.location (Transformation|GetRelativeTransform (Variables|Default|GetStaticMesh)))) 0.0) (Variables|Default|GetToBeDestroyed)))
      (Actor|DestroyActor :!label _label))
    (else
      (goto _label))))

(fn ConstructionScript)